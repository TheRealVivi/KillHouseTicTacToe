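; BP_MainPlayer is the main player character Blueprint, keeping its nameplate widget in sync with the player's stats.
; Tick runs through a 0.2-second Delay, throttling calls to AddNamePlates instead of updating every frame.
; AddNamePlates pushes health, experience and stamina ratios, plus name, level, points earned and wins as text, to the Nameplate component's widget through UpdateProgressMessage.
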(event Custom|AddNamePlates
  (Class|BPUI|UpdateProgress(Message) (UserInterface|GetUserWidgetObject (Variables|Default|GetNameplate)) (/ (Variables|Default|GetHealth) (Variables|Default|GetMaxHealth)) (/ (Variables|Default|GetExp) (Variables|Default|GetMaxExp)) (/ (Variables|Default|GetStamina) (Variables|Default|GetMaxStamina)) (Utilities|Text|ToText(String) (Variables|Default|GetName)) (Utilities|Text|ToText(Integer) (Variables|Default|GetLevel)) (Utilities|Text|ToText(Integer) (Variables|Default|GetPointsEarned)) (Utilities|Text|ToText(Integer) (Variables|Default|GetWins))))

(event EventBeginPlay)

(event Collision|EventActorBeginOverlap
  (params (OtherActor :type Actor%20Object%20Reference)))

(event EventTick
  (params (DeltaSeconds :type Float%20%28single-precision%29))
  (Utilities|FlowControl|Delay 0.2)
  (CallFunction|AddNamePlates))

(fn ConstructionScript)