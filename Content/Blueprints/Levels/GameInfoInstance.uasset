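; Game instance Blueprint that manages menu widgets and multiplayer sessions, adapted from an Unreal Engine tutorial.
; Main menu, host menu and loading screen widgets are created once and reused, while the server menu is rebuilt each time.
; Hosting creates a session and opens the Test level as a listen server; joining and destroying sessions are also handled.
; Failures route to DisplayErrorMessage, but it and both error-to-string helpers are empty stubs.
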(event Custom|OpenMainMenu
  (bind _returnvalue (Game|GetPlayerController 0))
  ;[1 1 1] Launch mainmenu and show mouse cursor (From Unreal Engine tutorial)
  (Utilities|IsValid (Variables|Widgets|GetMainMenu_WB)
    (:Is%20Valid
      _)
    (:Is%20Not%20Valid
      (bind _returnvalue_2 (UserInterface|CreateWidget "/Game/UI/Menus/MainMenu.MainMenu_C" _returnvalue))
      (Variables|Widgets|SetMainMenu_WB _returnvalue_2)))
  (UserInterface|Viewport|AddtoViewport (Variables|Widgets|GetMainMenu_WB) 0)
  (Variables|/Script/Engine.PlayerController|SetbShowMouseCursor _returnvalue true))

(event Custom|LaunchHostMenu
  ;[1 1 1] Launch host menu (From Unreal Engine tutorial)
  (Utilities|IsValid (Variables|Widgets|GetHostMenu_WB)
    (:Is%20Valid
      _)
    (:Is%20Not%20Valid
      (bind _returnvalue (UserInterface|CreateWidget "/Game/UI/Menus/HostMenu.HostMenu_C" (Game|GetPlayerController 0)))
      (Variables|Widgets|SetHostMenu_WB _returnvalue)))
  (UserInterface|Viewport|AddtoViewport (Variables|Widgets|GetHostMenu_WB) 0))

(event Custom|LaunchServerMenu
  ;[1 1 1] Create and launch a new server menu each time (From Unreal Engine tutorial)
  (bind _returnvalue (UserInterface|CreateWidget "/Game/UI/Menus/ServerMenu.ServerMenu_C" (Game|GetPlayerController 0)))
  (UserInterface|Viewport|AddtoViewport _returnvalue 0))

(event Custom|LaunchLobby
  (params (NumberOfPlayers :type Integer) (EnableLan :type Boolean) (ServerName :type Text))
  ;[1 1 1] Launch Tutorial Lobby (From Unreal Engine Tutorial)
  (Variables|ServerSettings|SetMaxPlayers NumberOfPlayers)
  (Variables|ServerSettings|SetServerName ServerName)
  (CallFunction|ShowLoadingScreen)
  (|Session (Game|GetPlayerController 0) (Variables|ServerSettings|GetMaxPlayers) EnableLan
    (:OnSuccess
      (Game|OpenLevel(byName) "Test" true "listen"))
    (:OnFailure
      (Utilities|DisplayErrorMessage "Failed To Create Session."))))

(event Custom|ShowLoadingScreen
  ;[1 1 1] Shows loading screen. (From Unreal Engine Tutorial)
  (Utilities|IsValid (Variables|Widgets|GetLoadingScreen_WB)
    (:Is%20Valid
      _)
    (:Is%20Not%20Valid
      (bind _returnvalue (UserInterface|CreateWidget "/Game/UI/LoadingScreen.LoadingScreen_C" (Game|GetPlayerController 0)))
      (Variables|Widgets|SetLoadingScreen_WB _returnvalue)))
  (UserInterface|Viewport|AddtoViewport (Variables|Widgets|GetLoadingScreen_WB) 0))

(event Custom|JoinServer
  (params (SessionToJoin :type Blueprint%20Session%20Result%20Structure))
  ;[1 1 1] Join Server (From Unreal Engine Tutorial)
  (CallFunction|ShowLoadingScreen)
  (|JoinSession (Game|GetPlayerController 0) SessionToJoin
    (:OnFailure
      (Utilities|DisplayErrorMessage "Failed to join session."))))

(event Custom|DestroySessionCaller
  (params (Player%20Controller :type Player%20Controller%20Object%20Reference))
  ;[1 1 1] Destroy session when called (From Unreal Engine Tutorial)
  (|DestroySession Player%20Controller))

(event EventHandleNetworkError
  (params (FailureType :type ENetworkFailure%20Enum :default "NetDriverAlreadyExists") (bIsServer :type Boolean))
  ;[1 1 1] Handle Network Errors and Display Message (From Unreal Engine Tutorial)
  (if (not bIsServer)
    (Utilities|DisplayErrorMessage (CallFunction|NetErrortoString FailureType))))

(event EventHandleTravelError
  (params (FailureType :type ETravelFailure%20Enum :default "NoLevel"))
  ;[1 1 1] Handle Travel Errors and Display Message (From Unreal Engine Tutorial)
  (Utilities|DisplayErrorMessage (CallFunction|TravelErrortoString FailureType)))

(fn NetErrortoString
  (params (FailureType :type ENetworkFailure%20Enum :default "NetDriverAlreadyExists"))
  (return ""))

(fn TravelErrortoString
  (params (FailureType :type ETravelFailure%20Enum :default "NoLevel"))
  (return ""))